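; Rocket component handler that periodically spawns BP_Rocket_Component actors at map locations below a spawn zone.
; BeginPlay starts a looping one-second timer and stores a hit ignore list from a helper that is currently empty.
; Each tick of the timer line-traces downward from the zone, spawning at the hit or printing a failure.
; GetRandomPointOnSurface holds random bounds math, but those nodes are unconnected.
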(event Custom|Event%20Spawn%20Component
  (bind _componentspawnzone (Variables|Default|GetComponentSpawnZone))
  (bind (_x _y _z) (|GetRandomPointOnSurface _componentspawnzone))
  (bind (_outhit _returnvalue) (Collision|LineTraceByChannel (Math|Vector|MakeVector _x _y _z) (Math|Vector|MakeVector _x _y -1.0) "TraceTypeQuery1" false (Variables|Default|GetHit%20Ignore%20List) "Persistent"))
  (if _returnvalue
    (bind _returnvalue_2 (Game|SpawnActorfromClass "/Game/RocketComponents/Blueprints/BP_Rocket_Component.BP_Rocket_Component_C" (Math|Transform|MakeTransform (.Location (Collision|BreakHitResult _outhit))) "Undefined" 0 0))
    (Default|GetComponent _returnvalue_2)
    (else
      (Development|PrintString "Line Trace failed to detect Map" true true "(R=1.000000,G=0.000000,B=0.000000,A=1.000000)" 1e+01))))

(event EventBeginPlay
  (Utilities|Time|SetTimerbyEvent (delegate Custom|Event%20Spawn%20Component) 1.0 true)
  (bind _ignore_list (CallFunction|CreateHitIgnoreList))
  (Variables|Default|SetHit%20Ignore%20List _ignore_list))

(fn ConstructionScript)

(fn CreateHitIgnoreList
  (return 0))