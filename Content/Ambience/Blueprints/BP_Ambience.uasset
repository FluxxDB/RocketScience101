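; BP_Ambience is an actor that plays and controls the menu ambience audio.
; ToggleMenu flips IsInMenu, starting the MenuAmbience audio component with a short logarithmic fade to AppliedVolume, or fading it out and stopping it after a delay.
; The track starts stopped on BeginPlay and replays when finished while in the menu.
; UpdateMenuVolume sets the volume multiplier, and an optional Tick debug printout shows volume and playing state.
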(event OnAudioFinished(MenuAmbience)
  (if (Variables|Default|GetIsInMenu)
    (Audio|Components|Audio|Play (Variables|Default|GetMenuAmbience) 0.0)))

(event EventBeginPlay
  (Audio|Components|Audio|Stop (Variables|Default|GetMenuAmbience)))

(event EventTick
  (params (DeltaSeconds :type Float%20%28single-precision%29))
  (bind _menuambience (Variables|Default|GetMenuAmbience))
  (if (Variables|Default|GetDebugMessageEnabled)
    (Development|PrintString (Utilities|String|Append (Utilities|String|MakeLiteralString "MenuAmbience Volume: ") (Utilities|String|ToString(Float) (Variables|/Script/Engine.AudioComponent|GetVolumeMultiplier _menuambience))) true true "(R=0.000000,G=0.660000,B=1.000000,A=1.000000)" DeltaSeconds)
    (Development|PrintString (Utilities|String|Append (Utilities|String|MakeLiteralString "MenuAmbience is playing: ") (Utilities|String|ToString(Boolean) (Audio|Components|Audio|IsPlaying _menuambience))) true true "(R=0.000000,G=0.660000,B=1.000000,A=1.000000)" DeltaSeconds)))

(fn ConstructionScript)

(fn UpdateMenuVolume
  (params (NewParam :type Float%20%28double-precision%29))
  (Audio|Components|Audio|SetVolumeMultiplier (Variables|Default|GetMenuAmbience) NewParam :!class /Script/Engine.AudioComponent))

(fn ToggleMenu
  (bind _menuambience (Variables|Default|GetMenuAmbience))
  (bind _menuambience_2 (Variables|Default|GetMenuAmbience))
  (if (Variables|Default|GetIsInMenu)
    (Variables|Default|SetIsInMenu false)
    (Audio|Components|Audio|AdjustVolume _menuambience_2 0.5 0.0 "Logarithmic" :!class /Script/Engine.AudioComponent)
    (Audio|Components|Audio|StopDelayed _menuambience_2 0.5)
    (else
      (Variables|Default|SetIsInMenu true)
      (Audio|Components|Audio|Play _menuambience 0.0)
      (Audio|Components|Audio|AdjustVolume _menuambience 0.5 (Variables|Default|GetAppliedVolume) "Logarithmic" :!class /Script/Engine.AudioComponent))))